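; BP_TetrisBoard is the Tetris board Blueprint, and its graph handles the score display for the game.
; On BeginPlay it creates a TetrisHUD widget, adds it to the viewport and binds a handler to OnPointsChanged.
; That handler writes CurrentScore with a "Points:" prefix into the HUD's Points text, so updates are event-driven.
; No board or piece logic is in this graph.
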(event Custom|OnPointsChanged_Event
  (Rendering|Components|TextRender|SetText (Variables|/Game/Tetris/TetrisHUD.TetrisHUD_C|GetPoints (Variables|Default|GetHUDWidget)) (Utilities|Text|ToText(String) (Utilities|String|Append (Utilities|String|MakeLiteralString "Points: ") (Utilities|String|ToString(Integer) (Variables|Default|GetCurrentScore))))))

(event EventBeginPlay
  (bind _returnvalue (UserInterface|CreateWidget "/Game/Tetris/TetrisHUD.TetrisHUD_C"))
  (bind _output_get (Variables|Default|SetHUDWidget _returnvalue))
  (UserInterface|Viewport|AddtoViewport _output_get 0)
  (EventDispatchers|BindEventtoOnPointsChanged (delegate Custom|OnPointsChanged_Event)))

(event Collision|EventActorBeginOverlap
  (params (OtherActor :type Actor%20Object%20Reference)))

(event EventTick
  (params (DeltaSeconds :type Float%20%28single-precision%29)))

(fn ConstructionScript)